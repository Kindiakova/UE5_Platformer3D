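; BP_MovingPlatfomr is a moving platform that shuttles back and forth along its local Y axis, starting on BeginPlay.
; A timeline track sets the Platform component's relative Y while keeping its current X and Z.
; The Move event flips a ReachedEnd flag to alternate Play and Reverse, and the timeline's Finished output calls Move again to loop the motion.
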(event Custom|Move
  (bind _platform (Variables|Default|GetPlatform))
  (bind _relativelocation (Variables|/Script/Engine.SceneComponent|GetRelativeLocation _platform))
  (if (not (Variables|Default|GetbReachedEnd))
    (Variables|Default|SetbReachedEnd true)
    (bind _newtrack_1 (Timeline|Timeline Play)
      (:Update
        (Transformation|SetRelativeLocation _platform (Math|Vector|MakeVector (.x _relativelocation) _newtrack_1 (.z _relativelocation)) false false))
      (:Finished
        (CallFunction|Move)))
    (else
      (Variables|Default|SetbReachedEnd false)
      (Timeline|Timeline Reverse))))

(event EventBeginPlay
  (CallFunction|Move))

(fn ConstructionScript)