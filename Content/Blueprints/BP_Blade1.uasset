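; BP_Blade1 is a swinging blade hazard that sends DieMessage to any actor overlapping its collision.
; From BeginPlay, a Move event waits a set delay, then plays or reverses a timeline based on the ReachedEnd flag.
; The timeline drives the pivot's pitch, keeping roll and yaw, and calls Move again on finish, so the motion repeats back and forth.
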(event OnComponentBeginOverlap(Collision)
  (params (OverlappedComponent :type Primitive%20Component%20Object%20Reference) (OtherActor :type Actor%20Object%20Reference) (OtherComp :type Primitive%20Component%20Object%20Reference) (OtherBodyIndex :type Integer) (bFromSweep :type Boolean) (SweepResult :type Hit%20Result%20Structure%20%28by%20ref%29))
  (Class|BPIPlayer|Die(Message) OtherActor))

(event Custom|Move
  (bind _pivot (Variables|Default|GetPivot))
  (bind _relativerotation (Variables|/Script/Engine.SceneComponent|GetRelativeRotation _pivot))
  (Utilities|FlowControl|Delay (Variables|Default|GetDelay))
  (if (not (Variables|Default|GetReachedEnd))
    (Variables|Default|SetReachedEnd true)
    (bind _newtrack_0 (Timeline|Timeline Play)
      (:Update
        (Transformation|SetRelativeRotation _pivot (Math|Rotator|MakeRotator (.roll _relativerotation) _newtrack_0 (.yaw _relativerotation)) false false))
      (:Finished
        (CallFunction|Move)))
    (else
      (Variables|Default|SetReachedEnd false)
      (Timeline|Timeline Reverse))))

(event EventBeginPlay
  (CallFunction|Move))

(fn ConstructionScript)